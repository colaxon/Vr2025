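; Cannon actor Blueprint with rotation pivots for the barrel and a lever, plus a shooting point for projectiles.
; A timeline is set up to rotate the cannon pivot and, on finish, spawn an enlarged Projectile at the shooting point's transform.
; The logic is unfinished: nothing triggers the timelines or lever rotation, and both rotation calls use zero rotation.
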(event `self.ReceiveBeginPlay`)

(fn `UserConstructionScript`)